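; BP_Bumper is a bumper that knocks a BP_Ball away when the ball overlaps it.
; Bump applies a velocity-change impulse pointing from the bumper to the ball, scaled by KnockbackForce, and plays an attached hit sound.
; The BumpLerp timeline moves the mechanism along Z and drives the point light's intensity and an emissive boost on a dynamic top material created in the construction script.
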(event Custom|Bump
  (params (Ball_BP :type BP%20Ball%20Object%20Reference))
  (Physics|AddImpulse (Variables|/Game/Blueprints/BP_Ball.BP_Ball_C|GetBall Ball_BP) (* (Math|Vector|GetUnitDirection(Vector) (Transformation|GetActorLocation) (Transformation|GetActorLocation Ball_BP)) (Variables|Default|GetKnockbackForce)) "None" true)
  (Audio|SpawnSoundAttached "/Game/Assets/Sounds/BumperHit.BumperHit" (Variables|Default|GetBumperMesh) "None" "0, 0, 0" "0, 0, 0" "KeepRelativeOffset" false 1.0 1.0 0.0 0 0)
  (bind _bumpalpha (Timeline|BumpLerp PlayFromStart)
    (:Update
      (Transformation|SetRelativeLocation (Variables|Default|GetBumperMechanism) (Math|Vector|Lerp(Vector) "0, 0, 0" "0, 0,-70.000000" _bumpalpha) false false)
      (Rendering|Components|Light|SetIntensity (Variables|Default|GetPointLight) (Math|Float|Lerp 0.0 5e+03 _bumpalpha))
      (Rendering|Material|SetScalarParameterValue (Variables|Default|GetBumperTopMID) "EmissiveBoost" (Math|Float|Lerp 0.0 2e+01 _bumpalpha) :!class /Script/Engine.MaterialInstanceDynamic))))

(event EventBeginPlay)

(event Collision|EventActorBeginOverlap
  (params (OtherActor :type Actor%20Object%20Reference))
  (bind _asbp_ball (Utilities|Casting|CastToBP_Ball OtherActor))
  (CallFunction|Bump _asbp_ball))

(event EventTick
  (params (DeltaSeconds :type Float%20%28single-precision%29)))

(fn ConstructionScript
  (bind _returnvalue (Rendering|Material|CreateDynamicMaterialInstance (Variables|Default|GetBumperMesh) 1 0 "None" :!class /Script/Engine.PrimitiveComponent))
  (Variables|Default|SetBumperTopMID _returnvalue))