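; Physics-driven ball actor that rolls on a table surface, with all logic running on Tick.
; Each frame it applies a delta-scaled DefaultSpeed velocity-change impulse to the Ball component.
; A downward line trace, left with persistent debug drawing, supplies the surface normal for an opposing TableStickyness impulse that presses the ball onto the table.
; It then resets the actor to a hard-coded height, keeping X and Y.
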(event EventBeginPlay)

(event Collision|EventActorBeginOverlap
  (params (OtherActor :type Actor%20Object%20Reference)))

(event EventTick
  (params (DeltaSeconds :type Float%20%28single-precision%29))
  (bind _returnvalue (Transformation|GetActorLocation))
  (bind _returnvalue_2 (Transformation|GetActorLocation))
  (Physics|AddImpulse (Variables|Default|GetBall) (* (Variables|Default|GetDefaultSpeed) DeltaSeconds) "None" true)
  (bind _outhit (Collision|LineTraceByChannel _returnvalue_2 (- _returnvalue_2 "0, 0,500.000000") "TraceTypeQuery1" false 0 "Persistent"))
  (Physics|AddImpulse (Variables|Default|GetBall) (* (* (.ImpactNormal (Collision|BreakHitResult _outhit)) -1) (* DeltaSeconds (Variables|Default|GetTableStickyness))) "None" false)
  (Transformation|SetActorLocation (Math|Vector|MakeVector (.x _returnvalue) (.y _returnvalue) -49.749901) false false))

(fn ConstructionScript)